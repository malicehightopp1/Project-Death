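; Test player character Blueprint that handles walking, looking and sprinting.
; BeginPlay adds the Enhanced Input mapping context; IA_Move moves relative to control yaw and IA_Look drives controller yaw and pitch.
; Raw Left Shift key events switch TargetSpeed between sprint and walk values, outside the Enhanced Input actions.
; Tick interpolates MaxWalkSpeed toward that target for smooth speed changes and prints it for debugging.
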(event `Key|LeftShift`
  (params (Key :type "Key Structure"))
  ; Sprinting
  (:`Pressed`
    (set `self.TargetSpeed` 600.0))
  (:`Released`
    (set `self.TargetSpeed` 300.0)))

(event `EnhancedInput|/Game/_MyFiles/Inputs/LocomotionInputs/IA_Move`
  (params (ActionValue :type "Vector2D Structure") (ElapsedSeconds :type "Float (double-precision)") (TriggeredSeconds :type "Float (double-precision)") (InputAction :type "InputAction Object Reference" :default "/Game/_MyFiles/Inputs/LocomotionInputs/IA_Move.IA_Move"))
  (bind (_returnvalue_roll _returnvalue_pitch _returnvalue_yaw) (`KismetMathLibrary.BreakRotator` (`self.GetControlRotation`)))
  ; Player movement
  (:`Triggered`
    (`self.AddMovementInput` (`KismetMathLibrary.GetForwardVector` (`KismetMathLibrary.MakeRotator` 0.0 0.0 _returnvalue_yaw)) ActionValue_X)
    (`self.AddMovementInput` (`KismetMathLibrary.GetRightVector` (`KismetMathLibrary.MakeRotator` 0.0 0.0 _returnvalue_yaw)) ActionValue_Y)))

(event `self.ReceiveBeginPlay`
  ; Grabbing enhanced input system
  (`EnhancedInputSubsystemInterface.AddMappingContext` (pcsubsystem `EnhancedInputLocalPlayerSubsystem` (`GameplayStatics.GetPlayerController` 0)) "/Game/_MyFiles/Inputs/InputMappingContexts/IMC_PlayerInput.IMC_PlayerInput" 0 (struct)))

(event `self.ReceiveTick`
  (params (DeltaSeconds :type "Float (single-precision)"))
  (bind _charactermovement (`self.CharacterMovement`))
  ; Lerping values for smoother stops and starts for sprinting
  (bind _output_get (set `CharacterMovementComponent.MaxWalkSpeed` (`KismetMathLibrary.FInterpTo` (`CharacterMovementComponent.MaxWalkSpeed` _charactermovement) (`self.TargetSpeed`) DeltaSeconds (`self.SmoothingSpeed`)) _charactermovement))
  ; Testing
  (`KismetSystemLibrary.PrintString` (`KismetStringLibrary.Conv_DoubleToString` _output_get)))

(event `EnhancedInput|/Game/_MyFiles/Inputs/LocomotionInputs/IA_Look`
  (params (ActionValue :type "Vector2D Structure") (ElapsedSeconds :type "Float (double-precision)") (TriggeredSeconds :type "Float (double-precision)") (InputAction :type "InputAction Object Reference" :default "/Game/_MyFiles/Inputs/LocomotionInputs/IA_Look.IA_Look"))
  ; Camera rotation
  (:`Triggered`
    (bind _result (`/Engine/EditorBlueprintResources/StandardMacros.NegateFloat` ActionValue_X)
      (:`  `
        (`self.AddControllerYawInput` _result)
        (`self.AddControllerPitchInput` ActionValue_Y)))))

(fn `UserConstructionScript`)